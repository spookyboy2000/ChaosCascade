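; BP_MyPlayer1 is a player Blueprint, apparently a test, with a debug marker and basic damage handling.
; BeginPlay and Tick draw a cyan debug circle, with zeroed axes, at the actor's location offset along world X by LocationXFloat.
; AnyDamage adds damage to Health rather than subtracting it, destroying the actor only when Health equals exactly 20.
; The capsule overlap event is empty, and a Niagara test cast and subtractive health check are unconnected.
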(event OnComponentBeginOverlap(CapsuleComponent)
  (params (OverlappedComponent :type Primitive%20Component%20Object%20Reference) (OtherActor :type Actor%20Object%20Reference) (OtherComp :type Primitive%20Component%20Object%20Reference) (OtherBodyIndex :type Integer) (bFromSweep :type Boolean) (SweepResult :type Hit%20Result%20Structure%20%28by%20ref%29)))

(event EventBeginPlay
  (bind _returnvalue (Transformation|GetActorLocation))
  (Rendering|Debug|DrawDebugCircle (Math|Vector|MakeVector (+ (.x _returnvalue) (Variables|Default|GetLocationXFloat)) (.y _returnvalue) (.z _returnvalue)) 1e+01 12 "(R=0.000000,G=0.970476,B=1.000000,A=1.000000)" 0.0 5.0 "0.000000,0.000000,0.000000" "0.000000,0.000000,0.000000"))

(event EventTick
  (params (DeltaSeconds :type Float%20%28single-precision%29))
  (bind _returnvalue (Transformation|GetActorLocation))
  (Rendering|Debug|DrawDebugCircle (Math|Vector|MakeVector (+ (.x _returnvalue) (Variables|Default|GetLocationXFloat)) (.y _returnvalue) (.z _returnvalue)) 1e+01 12 "(R=0.000000,G=0.970476,B=1.000000,A=1.000000)" 0.0 5.0 "0.000000,0.000000,0.000000" "0.000000,0.000000,0.000000"))

(event Game|Damage|EventAnyDamage
  (params (Damage :type Float%20%28single-precision%29) (DamageType :type Damage%20Type%20Object%20Reference) (InstigatedBy :type Controller%20Object%20Reference) (DamageCauser :type Actor%20Object%20Reference))
  (bind _output_get (Variables|Default|SetHealth (+ (Variables|Default|GetHealth) Damage)))
  (if (== _output_get 2e+01)
    (Actor|DestroyActor)))

(fn ConstructionScript)