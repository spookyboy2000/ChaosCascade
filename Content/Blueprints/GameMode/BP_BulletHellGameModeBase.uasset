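; Game mode Blueprint for a bullet hell game that sets up the view and HUD when play begins.
; BeginPlay spawns BP_Camera at a fixed raised transform, makes it the first player's view target, then creates WB_Interface, stores it and adds it to the viewport.
; Tick looks up the Player1 actor, but the debug box drawing its MaxBoundary is disconnected and never runs.
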(event EventBeginPlay
  (bind _returnvalue (Game|SpawnActorfromClass "/Game/Blueprints/GameMode/BP_Camera.BP_Camera_C" (Math|Transform|MakeTransform "0.000000,0.000000,1500.000000" "-90.000000,180.000000,180.000000") "Undefined" "MultiplyWithRoot" 0 0))
  (Game|Player|SetViewTargetwithBlend (Game|GetPlayerController (Variables|/Script/Engine.Pawn|GetPlayerState (Game|GetPlayerCharacter 0))) _returnvalue 0.0 "VTBlend_Linear" 0.0 false)
  (bind _returnvalue_2 (UserInterface|CreateWidget "/Game/Blueprints/GameMode/WB_Interface.WB_Interface_C"))
  (bind _output_get (Variables|Default|SetHeadsUpDisplay_UI _returnvalue_2))
  (UserInterface|Viewport|AddtoViewport _output_get 0))

(event EventTick
  (params (DeltaSeconds :type Float%20%28single-precision%29))
  (bind _returnvalue (Actor|GetActorOfClass "/Script/BulletHell.Player1")))

(fn ConstructionScript)