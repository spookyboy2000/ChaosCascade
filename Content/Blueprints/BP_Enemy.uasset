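; BP_Enemy is an enemy actor that roams between randomly ordered BP_Location actors at a fixed height.
; On BeginPlay it shuffles those locations, then the Speed timeline lerps it toward the current one, re-basing the start point every update.
; Each finished move advances the index and replays after a delay, reshuffling when the last index is reached.
; The Bullets event is empty, and a BP_Niagara_Test2 spawn node is left unconnected.
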(event Custom|Bullets)

(event EventBeginPlay
  (bind _returnvalue (Transformation|GetActorLocation))
  (bind _returnvalue_2 (Transformation|GetActorLocation))
  (CallFunction|Bullets)
  (Variables|Default|SetSpawnLocation_0 (Math|Vector|MakeVector (.x _returnvalue) (.y _returnvalue) 5.0))
  (bind _outactors (Actor|GetAllActorsOfClass "/Game/Blueprints/BP_Location.BP_Location_C"))
  (Utilities|Array|Shuffle _outactors)
  (bind _newtrack_0 (Timeline|Speed Play)
    (:Update
      (Transformation|SetActorLocation (Math|Vector|MakeVector (.x (Math|Vector|Lerp(Vector) (Math|Vector|MakeVector (.x (Variables|Default|GetSpawnLocation_0)) (.y (Variables|Default|GetSpawnLocation_0)) 5.0) (Math|Vector|MakeVector (.x (Transformation|GetActorLocation (Utilities|Array|Get(acopy) _outactors (stale _output_get)))) (.y (Transformation|GetActorLocation (Utilities|Array|Get(acopy) _outactors (stale _output_get)))) 5.0) _newtrack_0)) (.y (Math|Vector|Lerp(Vector) (Math|Vector|MakeVector (.x (Variables|Default|GetSpawnLocation_0)) (.y (Variables|Default|GetSpawnLocation_0)) 5.0) (Math|Vector|MakeVector (.x (Transformation|GetActorLocation (Utilities|Array|Get(acopy) _outactors (stale _output_get)))) (.y (Transformation|GetActorLocation (Utilities|Array|Get(acopy) _outactors (stale _output_get)))) 5.0) _newtrack_0)) 5.0) false false)
      (Variables|Default|SetSpawnLocation_0 (Math|Vector|MakeVector (.x _returnvalue_2) (.y _returnvalue_2) 5.0))
      (if (== (stale _output_get) (- (Utilities|Array|Length _outactors) 1))
        (Utilities|Array|Shuffle _outactors)
        (Variables|Default|Setint 0)))
    (:Finished
      (bind _output_get (Variables|Default|Setint (+ (stale _output_get) 1)))
      (Utilities|FlowControl|Delay 3.0)
      (Timeline|Speed PlayFromStart))))

(fn ConstructionScript)