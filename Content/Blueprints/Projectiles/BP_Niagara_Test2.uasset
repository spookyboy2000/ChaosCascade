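; Test projectile actor that turns Niagara particles into damage sources by registering itself as the system's BPCALLBACK export handler.
; ParticleData sphere-traces each exported particle a short way along its velocity, sized by the particle, and damages the hit actor.
; The same event also damages player pawn 0 unconditionally before the loop.
; A Bullets event spawns another copy of the actor; leftover print and destroy logic is unwired.
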(event Custom|Bullets
  (bind _returnvalue (Game|SpawnActorfromClass "BP_Niagara_Test2_C" (Transformation|GetActorTransform) "Undefined" "MultiplyWithRoot" self 0)))

(event EventTick
  (params (DeltaSeconds :type Float%20%28single-precision%29)))

(event EventBeginPlay
  (Class|NiagaraComponent|SetVariableObject (Variables|Default|GetNiagara) "BPCALLBACK" self))

(event EventParticleData
  (params (Data :type Array%20of%20Basic%20Particle%20Data%20Structures) (NiagaraSystem :type Niagara%20System%20Object%20Reference) (SimulationPositionOffset :type Vector%20%28by%20ref%29 :default "0, 0, 0"))
  (Game|Damage|ApplyDamage (Game|Player|GetPlayerPawn 0) 2e+01 0 0)
  (for _array_element 0
    (bind _outhit (Collision|SphereTraceByChannel (.Position (Utilities|Struct|BreakBasicParticleData _array_element)) (+ (.Position (Utilities|Struct|BreakBasicParticleData _array_element)) (* (.Velocity (Utilities|Struct|BreakBasicParticleData _array_element)) 0.1)) (.Size (Utilities|Struct|BreakBasicParticleData _array_element)) "TraceTypeQuery1" false 0 "None"))
    (Game|Damage|ApplyDamage (.HitActor (Collision|BreakHitResult _outhit)) 2e+01 0 0)))

(fn ConstructionScript)