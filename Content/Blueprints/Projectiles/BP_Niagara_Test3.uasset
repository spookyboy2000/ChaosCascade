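; BP_Niagara_Test3 is a test projectile Blueprint that turns Niagara particle callbacks into damage on the player.
; On BeginPlay it registers itself as the Niagara system's BPCALLBACK object to receive exported particle data.
; Each ParticleData callback applies fixed damage directly to the first player pawn, without reading particle positions.
; An unconnected loop that would sphere-trace along each particle's velocity and damage the hit actor never runs.
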(event EventBeginPlay
  (Class|NiagaraComponent|SetVariableObject (Variables|Default|GetNiagara) "BPCALLBACK" self))

(event EventParticleData
  (params (Data :type Array%20of%20Basic%20Particle%20Data%20Structures) (NiagaraSystem :type Niagara%20System%20Object%20Reference) (SimulationPositionOffset :type Vector%20%28by%20ref%29 :default "0, 0, 0"))
  (Game|Damage|ApplyDamage (Game|Player|GetPlayerPawn 0) 2e+01 0 0))

(fn ConstructionScript)